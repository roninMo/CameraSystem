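; BP_CameraManager is a camera manager Blueprint with hooks for first-person, third-person, third-person aiming, target-lock and spectator camera behaviors.
; Each behavior override and the view-target update simply forwards to its parent implementation, so the camera logic lives in the parent class.
; BlueprintUpdateCamera returns false with zeroed outputs, and the construction script is empty, leaving the asset as a pass-through shell.
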(fn ConstructionScript)

(fn FirstPersonCameraBehavior
  (params (DeltaTime :type Float%20%28single-precision%29))
  (bind _outvt (|CallParentFunction DeltaTime))
  (return _outvt))

(fn BlueprintUpdateCamera
  (params (CameraTarget :type Actor%20Object%20Reference))
  (return "0, 0, 0" "0, 0, 0" 0.0 false))

(fn BPUpdateViewTarget
  (params (DeltaTime :type Float%20%28single-precision%29))
  (bind (_outvt _bapplymodifiers) (|CallParentFunction DeltaTime))
  (return _outvt _bapplymodifiers))

(fn SpectatorCameraBehavior
  (params (DeltaTime :type Float%20%28single-precision%29))
  (bind _outvt (|CallParentFunction DeltaTime))
  (return _outvt))

(fn ThirdPersonAimingCameraBehavior
  (params (DeltaTime :type Float%20%28single-precision%29))
  (bind _outvt (|CallParentFunction DeltaTime))
  (return _outvt))

(fn TargetLockCameraBehavior
  (params (DeltaTime :type Float%20%28single-precision%29))
  (bind _outvt (|CallParentFunction DeltaTime))
  (return _outvt))

(fn ThirdPersonCameraBehavior
  (params (DeltaTime :type Float%20%28single-precision%29))
  (bind _outvt (|CallParentFunction DeltaTime))
  (return _outvt))