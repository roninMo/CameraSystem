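; Blueprint camera manager that exposes per-mode camera behaviors: first person, third person, third-person aiming, target lock and spectator.
; Each behavior override passes DeltaTime to its parent implementation and returns the result unchanged, so all camera logic comes from the parent class.
; BlueprintUpdateCamera returns false with zeroed outputs, and the UpdateViewTarget event and construction script are empty.
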(event EventUpdateViewTarget
  (params (OutVT :type T%20View%20Target%20Structure%20%28by%20ref%29) (DeltaTime :type Float%20%28single-precision%29) (bApplyModifiers :type Boolean%20%28by%20ref%29)))

(fn ConstructionScript)

(fn FirstPersonCameraBehavior
  (params (DeltaTime :type Float%20%28single-precision%29))
  (bind _outvt (|CallParentFunction DeltaTime))
  (return _outvt))

(fn BlueprintUpdateCamera
  (params (CameraTarget :type Actor%20Object%20Reference))
  (return "0, 0, 0" "0, 0, 0" 0.0 false))

(fn TargetLockCameraBehavior
  (params (DeltaTime :type Float%20%28single-precision%29))
  (bind _outvt (|CallParentFunction DeltaTime))
  (return _outvt))

(fn ThirdPersonAimingCameraBehavior
  (params (DeltaTime :type Float%20%28single-precision%29))
  (bind _outvt (|CallParentFunction DeltaTime))
  (return _outvt))

(fn SpectatorCameraBehavior
  (params (DeltaTime :type Float%20%28single-precision%29))
  (bind _outvt (|CallParentFunction DeltaTime))
  (return _outvt))

(fn ThirdPersonCameraBehavior
  (params (DeltaTime :type Float%20%28single-precision%29))
  (bind _outvt (|CallParentFunction DeltaTime))
  (return _outvt))